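; BannaPeel is a banana peel hazard actor that briefly halts the BP_Vroomba1 character that runs into it.
; On box overlap it hides its mesh, zeroes the character's max walk speed, waits briefly, then calls ResetSpeed and destroys itself.
; ResetSpeed restores walk speed from the peel's own default variable, not the character's previous value.
; SetSpeed is not called here, and the acceleration changes in both functions are disconnected.
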(event `self.ReceiveBeginPlay`)

(event `self.Box.OnComponentBeginOverlap`
  (params (OverlappedComponent :type "PrimitiveComponent Object Reference") (OtherActor :type "Actor Object Reference") (OtherComp :type "PrimitiveComponent Object Reference") (OtherBodyIndex :type Integer) (bFromSweep :type Boolean) (SweepResult :type "HitResult Structure (by ref)"))
  (bind _asbp_vroomba_1 (cast `/Game/Jamifesto2023/Blueprints/BP_Vroomba1` OtherActor))
  (`SceneComponent.SetHiddenInGame` (`self.StaticMesh`) true false)
  (bind _charactermovement (`Character.CharacterMovement` _asbp_vroomba_1))
  (set `CharacterMovementComponent.MaxWalkSpeed` 0.0 _charactermovement)
  (`KismetSystemLibrary.Delay` 0.4)
  (`self.ResetSpeed` _charactermovement _charactermovement)
  (`self.K2_DestroyActor`))

(fn `ResetSpeed`
  (params (self2 :type "CharacterMovementComponent Object Reference") (self3 :type "CharacterMovementComponent Object Reference"))
  (`KismetSystemLibrary.PrintString` "RESET SPEED")
  (set `CharacterMovementComponent.MaxWalkSpeed` (`self.WalkSpeedDeafult `) self2))

(fn `SetSpeed`
  (params (self2 :type "CharacterMovementComponent Object Reference") (self3 :type "CharacterMovementComponent Object Reference"))
  (set `CharacterMovementComponent.MaxWalkSpeed` (`self.Max Walk Speed`) self3))

(fn `UserConstructionScript`)