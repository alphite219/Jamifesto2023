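; Lap line for a Vroomba race that counts completed laps and resets the course for the next one.
; Any overlap on the line collision arms it by setting GameStart.
; A separate reset collision then increments a Vroomba's LapNumber if its checkpoint count matches CheckpointNumCheck.
; It then sends ResetCheckpoints interface messages to that Vroomba, checkpoints and spawners.
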(event `self.ReceiveBeginPlay`
  (`GameplayStatics.GetAllActorsOfClass` null))

(event `self.LineCollison.OnComponentBeginOverlap`
  (params (OverlappedComponent :type "PrimitiveComponent Object Reference") (OtherActor :type "Actor Object Reference") (OtherComp :type "PrimitiveComponent Object Reference") (OtherBodyIndex :type Integer) (bFromSweep :type Boolean) (SweepResult :type "HitResult Structure (by ref)"))
  (set `self.GameStart?` true))

(event `self.ResetCollision.OnComponentBeginOverlap`
  (params (OverlappedComponent :type "PrimitiveComponent Object Reference") (OtherActor :type "Actor Object Reference") (OtherComp :type "PrimitiveComponent Object Reference") (OtherBodyIndex :type Integer) (bFromSweep :type Boolean) (SweepResult :type "HitResult Structure (by ref)"))
  (if (`self.GameStart?`)
    (bind _asbp_vroomba_1 (cast `/Game/Jamifesto2023/Blueprints/BP_Vroomba1` OtherActor))
    (if (== (`self.CheckpointNumCheck`) (`/Game/Jamifesto2023/Blueprints/BP_Vroomba1.CheckpointNum` _asbp_vroomba_1))
      (`/Engine/EditorBlueprintResources/StandardMacros.IncrementInt` (`/Game/Jamifesto2023/Blueprints/BP_Vroomba1.LapNumber` _asbp_vroomba_1)
        (:`  `
          (`KismetSystemLibrary.PrintString` "Hello")
          (message `/Game/Jamifesto2023/Blueprints/Components/CheckpointInterface.ResetCheckpoints` _asbp_vroomba_1 null)
          (bind _outactors (`GameplayStatics.GetAllActorsOfClass` "/Game/Jamifesto2023/Blueprints/Components/Checkpoint.Checkpoint_C"))
          (message `/Game/Jamifesto2023/Blueprints/Components/CheckpointInterface.ResetCheckpoints` _outactors _asbp_vroomba_1)
          (bind _outactors_2 (`GameplayStatics.GetAllActorsOfClass` "/Game/Jamifesto2023/Blueprints/Components/Spawner.Spawner_C"))
          (message `/Game/Jamifesto2023/Blueprints/Components/CheckpointInterface.ResetCheckpoints` _outactors_2 null))))))

(fn `UserConstructionScript`)