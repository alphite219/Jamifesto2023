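; Battery pickup actor that gives an overlapping BP_Vroomba1 a temporary speed boost.
; A looping timer spins the Cylinder mesh until pickup hides it.
; Box overlap flags IsBoosting, sets max acceleration and adds to walk speed, then starts a looping countdown.
; Each countdown tick clears IsBoosting and prints the remaining time; at zero, stored default speeds are restored and the actor destroys itself.
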(event `self.ReceiveBeginPlay`
  (`KismetSystemLibrary.K2_SetTimer` null "Spin" 0.01 true)
  (set `self.Timer` (`self.MaxTimer`)))

(event `self.Box.OnComponentBeginOverlap`
  (params (OverlappedComponent :type "PrimitiveComponent Object Reference") (OtherActor :type "Actor Object Reference") (OtherComp :type "PrimitiveComponent Object Reference") (OtherBodyIndex :type Integer) (bFromSweep :type Boolean) (SweepResult :type "HitResult Structure (by ref)"))
  (bind _asbp_vroomba_1 (cast `/Game/Jamifesto2023/Blueprints/BP_Vroomba1` OtherActor))
  (set `/Game/Jamifesto2023/Blueprints/BP_Vroomba1.IsBoosting` true _asbp_vroomba_1)
  (bind _charactermovement (`Character.CharacterMovement` _asbp_vroomba_1))
  (`self.SetSpeed` _charactermovement _charactermovement)
  (`SceneComponent.SetHiddenInGame` (`self.Cylinder`) true false)
  (bind _returnvalue (`KismetSystemLibrary.K2_SetTimerDelegate` (delegate `Timer`) 0.1 true)))

(event `Timer`
  (set `/Game/Jamifesto2023/Blueprints/BP_Vroomba1.IsBoosting` false (stale `self.Box.OnComponentBeginOverlap` _asbp_vroomba_1))
  (if (> (`self.Timer`) 0.0)
    (bind _output_get (set `self.Timer` (- (`self.Timer`) 0.1)))
    (`KismetSystemLibrary.PrintString` (`KismetStringLibrary.Conv_DoubleToString` _output_get))
    (else
      (bind _charactermovement (`Character.CharacterMovement` (stale `self.Box.OnComponentBeginOverlap` _asbp_vroomba_1)))
      (`self.ResetSpeed` _charactermovement _charactermovement)
      (`KismetSystemLibrary.K2_PauseTimerHandle` (stale `self.Box.OnComponentBeginOverlap` _returnvalue))
      (`self.K2_DestroyActor`))))

(fn `ResetSpeed`
  (params (self2 :type "CharacterMovementComponent Object Reference") (self3 :type "CharacterMovementComponent Object Reference"))
  (`KismetSystemLibrary.PrintString` "RESET SPEED")
  (set `CharacterMovementComponent.MaxAcceleration` (`self.AccelerationDefault`) self3)
  (set `CharacterMovementComponent.MaxWalkSpeed` (`self.WalkSpeedDeafult `) self2)
  (set `self.Timer` (`self.MaxTimer`)))

(fn `SetSpeed`
  (params (self2 :type "CharacterMovementComponent Object Reference") (self3 :type "CharacterMovementComponent Object Reference"))
  (set `CharacterMovementComponent.MaxAcceleration` (`self.Max Acceleration`) self2)
  (set `CharacterMovementComponent.MaxWalkSpeed` (+ (`CharacterMovementComponent.MaxWalkSpeed` self3) 300.0) self3))

(fn `Spin`
  (`SceneComponent.K2_AddLocalRotation` (`self.Cylinder`) (struct :`Pitch` 0.5 :`Yaw` 2.0 :`Roll` -0.5) false false))

(fn `UserConstructionScript`)